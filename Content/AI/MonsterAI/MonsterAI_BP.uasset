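; MonsterAI_BP is an AI monster that chases the player and triggers a jumpscare when in attack range.
; TTK runs a 150-unit sphere trace for pawns, checks the Player tag, then calls Jumpscare and returns the result.
; Jumpscare plays a shutter sound, shakes the camera, blends the view to the monster and disables player input.
; It also exposes walk-speed and chase-audio controls; resumable audio is still a TODO.
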(event `Jumpscare`
  (bind _returnvalue (`GameplayStatics.GetPlayerController` 0))
  (`GameplayStatics.PlaySound2D` "/Engine/VREditor/Sounds/UI/Camera_Shutter.Camera_Shutter" 1.0 1.0 0.0 null null)
  (`PlayerCameraManager.StartCameraShake` :`self` (`GameplayStatics.GetPlayerCameraManager` 0) :`ShakeClass` "/Game/摄像机晃动/震屏.震屏_C" :`Scale` 0.1)
  (`PlayerController.SetViewTargetWithBlend` _returnvalue self 1.0 "VTBlend_Cubic" 0.0 false)
  (`self.DisableInput` (`GameplayStatics.GetPlayerPawn` 0) _returnvalue))

(event `播放追击音效`
  ;[1 1 1] 后续需要做一个计时器，如果玩家在3s内再次被追就按照上一次播放结束的地方继续播放
  (`AudioComponent.Play` (`self.追击音效`) 0.0))

(event `停止追击音效`
  ;[1 1 1] 后续需要做一个计时器，如果玩家在3s内再次被追就按照上一次播放结束的地方继续播放
  (`AudioComponent.Stop` (`self.追击音效`)))

(fn `SetMaxWalkSpeed`
  (params (NewSpeed :type "Float (double-precision)"))
  (set `CharacterMovementComponent.MaxWalkSpeed` NewSpeed (`self.CharacterMovement`)))

(fn `TTK`
  (returns (`追击是否成功` :type Boolean))
  (bind _returnvalue (`self.K2_GetActorLocation`))
  (bind (_outhit _returnvalue_2) (`KismetSystemLibrary.SphereTraceSingleForObjects` :`Start` _returnvalue :`End` _returnvalue :`Radius` 150.0 :`ObjectTypes` (`|MakeArray` "ObjectTypeQuery3" :!type "EObjectTypeQuery Enum") :`DrawDebugType` "ForOneFrame" :`TraceColor` (struct :`A` 1.0) :`TraceHitColor` (struct :`R` 1.0 :`B` 0.921747 :`A` 1.0))) ; AI移动到刺激对象附近后进行球体检测,判断对方是否在自己攻击范围内
  (if _returnvalue_2
    (if (`self.ActorHasTag` (`.HitActor` (`GameplayStatics.BreakHitResult` _outhit)) "Player")
      (`KismetSystemLibrary.PrintString` "TTK") ; 在攻击范围内执行攻击操作
      (`self.Jumpscare`)
      (return true)
      (else
        (`KismetSystemLibrary.PrintString` "TTK_F")
        (return false)))))

(fn `UserConstructionScript`)