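; Interactive door Blueprint that a Player-tagged actor can swing open and closed while standing in its trigger Box.
; Box begin and end overlaps enable or disable interaction on that actor and open or close a Gate that guards the interact event (交互).
; Each interaction that passes the Gate alternates through a FlipFlop, playing or reversing the OPENDOOR timeline, which lerps the Door's relative yaw through a quarter turn.
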(event `/Game/BP/ThirdPersonBP/Player_Intelface.交互`
  (`/Engine/EditorBlueprintResources/StandardMacros.Gate` true :!label _label
    (:`Exit`
      (`/Engine/EditorBlueprintResources/StandardMacros.FlipFlop`
        (:`A`
          (bind (_direction _alpha) (`Timeline|OPENDOOR` :!label _label_2)
            (:`Update`
              (`SceneComponent.K2_SetRelativeRotation` (`self.Door`) (`KismetMathLibrary.MakeRotator` 0.0 0.0 (`KismetMathLibrary.Lerp` 0.0 90.0 _alpha)) false false))))
        (:`B`
          (goto _label_2 :!via `Reverse`))))))

(event `self.Box.OnComponentBeginOverlap`
  (params (OverlappedComponent :type "PrimitiveComponent Object Reference") (OtherActor :type "Actor Object Reference") (OtherComp :type "PrimitiveComponent Object Reference") (OtherBodyIndex :type Integer) (bFromSweep :type Boolean) (SweepResult :type "HitResult Structure (by ref)"))
  (if (`self.ActorHasTag` OtherActor "Player")
    (`/Game/BP/PlayerFunctionLibrary.启用交互` self OtherActor)
    (goto _label :!via `Open`)))

(event `self.Box.OnComponentEndOverlap`
  (params (OverlappedComponent :type "PrimitiveComponent Object Reference") (OtherActor :type "Actor Object Reference") (OtherComp :type "PrimitiveComponent Object Reference") (OtherBodyIndex :type Integer))
  (if (`self.ActorHasTag` OtherActor "Player")
    (`/Game/BP/PlayerFunctionLibrary.禁用交互` OtherActor)
    (goto _label :!via `Close`)))

(fn `UserConstructionScript`)