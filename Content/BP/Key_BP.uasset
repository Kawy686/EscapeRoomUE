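; Key pickup actor that spins on its yaw axis through a timeline and gives the third-person character a key.
; Box overlap, gated by a DoOnce that resets on exit, snaps the key to the character's 拾取位 component and sets 是否拿到钥匙 if not already set.
; After a short delay the key destroys itself, a bug workaround according to its printed message, which says unlocking is unaffected.
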(event `self.ReceiveBeginPlay`
  (bind (_direction _alpha) (`Timeline|自旋转`)
    (:`Update`
      (`self.K2_SetActorRelativeRotation` (`KismetMathLibrary.MakeRotator` 0.0 0.0 (`KismetMathLibrary.Lerp` 0.0 360.0 _alpha))))))

(event `self.Box.OnComponentBeginOverlap`
  (params (OverlappedComponent :type "PrimitiveComponent Object Reference") (OtherActor :type "Actor Object Reference") (OtherComp :type "PrimitiveComponent Object Reference") (OtherBodyIndex :type Integer) (bFromSweep :type Boolean) (SweepResult :type "HitResult Structure (by ref)"))
  (bind _asthird_person_character (cast `/Game/BP/ThirdPersonBP/Blueprints/ThirdPersonCharacter` OtherActor))
  (`/Engine/EditorBlueprintResources/StandardMacros.DoOnce` false :!label _label
    (:`Completed`
      (if (not (`/Game/BP/ThirdPersonBP/Blueprints/ThirdPersonCharacter.是否拿到钥匙` _asthird_person_character))
        (`self.K2_AttachToComponent` (`/Game/BP/ThirdPersonBP/Blueprints/ThirdPersonCharacter.拾取位` _asthird_person_character) "None" "SnapToTarget" "SnapToTarget" "SnapToTarget")
        (set `/Game/BP/ThirdPersonBP/Blueprints/ThirdPersonCharacter.是否拿到钥匙` true _asthird_person_character)
        (`KismetSystemLibrary.Delay` 2.0)
        (`self.K2_DestroyActor`)
        (`KismetSystemLibrary.PrintText` "由于有BUG,拾取后会自动销毁钥匙,钥匙销毁不影响解锁。" true true (struct :`G` 0.66 :`B` 1.0 :`A` 1.0) 3.0)))))

(event `self.Box.OnComponentEndOverlap`
  (params (OverlappedComponent :type "PrimitiveComponent Object Reference") (OtherActor :type "Actor Object Reference") (OtherComp :type "PrimitiveComponent Object Reference") (OtherBodyIndex :type Integer))
  (cast `/Game/BP/ThirdPersonBP/Blueprints/ThirdPersonCharacter` OtherActor)
  (goto _label :!via `Reset`))

(fn `UserConstructionScript`)