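; Dropped-object Blueprint (掉落物体_BP) that plays impact and rolling sounds and reports noise events.
; Mesh overlap triggers a sphere trace that, on a hit, plays the drop sound and reports noise.
; Every Tick, fast Z-axis spin triggers the rolling sound, a louder noise and debug print, without checking the trace hit or throttling repeats.
; Both paths switch on surface type; the author flags the graph as buggy.
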(event `self.ReceiveTick`
  (params (DeltaSeconds :type "Float (single-precision)"))
  ;[1 1 1] 有BUG，得改
  (`self.滚动声音`))

(event `掉落声音`
  (bind _returnvalue (`SceneComponent.K2_GetComponentLocation` (`self.StaticMesh`)))
  ;[1 1 1] 有BUG，得改
  (bind (_outhit _returnvalue_2) (`KismetSystemLibrary.SphereTraceSingle` :`Start` _returnvalue :`End` _returnvalue :`Radius` 100.0 :`TraceChannel` "TraceTypeQuery1" :`DrawDebugType` "ForDuration"))
  (if _returnvalue_2
    (switch `EPhysicalSurface` (`GameplayStatics.GetSurfaceType` _outhit)
      (:`SurfaceType_Default`
        (bind (_bblockinghit _binitialoverlap _time _distance _location) (`GameplayStatics.BreakHitResult` _outhit))
        (`GameplayStatics.PlaySoundAtLocation` "/Engine/VREditor/Sounds/UI/Click_on_Button_Cue.Click_on_Button_Cue" _location (struct) 1.0 1.0 0.0 null null null)
        (`AISense_Hearing.ReportNoiseEvent` _location 1.0 null)))))

(event `滚动声音`
  (bind _returnvalue (`SceneComponent.K2_GetComponentLocation` (`self.StaticMesh`)))
  (bind (_returnvalue_x _returnvalue_y _returnvalue_z) (`KismetMathLibrary.BreakVector` (`PrimitiveComponent.GetPhysicsAngularVelocityInDegrees` (`self.StaticMesh`) "None")))
  ;[1 1 1] 有BUG，得改
  (if (> (`KismetMathLibrary.Abs` _returnvalue_z) 120.0)
    (bind _outhit (`KismetSystemLibrary.SphereTraceSingle` _returnvalue _returnvalue 100.0 "TraceTypeQuery1"))
    (if true
      (switch `EPhysicalSurface` (`GameplayStatics.GetSurfaceType` _outhit)
        (:`SurfaceType_Default`
          (bind (_bblockinghit _binitialoverlap _time _distance _location) (`GameplayStatics.BreakHitResult` _outhit))
          (`GameplayStatics.PlaySoundAtLocation` "/Engine/VREditor/Sounds/UI/Click_on_Button.Click_on_Button" _location (struct) 1.0 1.0 0.0 null null null)
          (`AISense_Hearing.ReportNoiseEvent` _location 3000.0 self)
          (`KismetSystemLibrary.PrintString` "滚动"))))))

(event `self.StaticMesh.OnComponentBeginOverlap`
  (params (OverlappedComponent :type "PrimitiveComponent Object Reference") (OtherActor :type "Actor Object Reference") (OtherComp :type "PrimitiveComponent Object Reference") (OtherBodyIndex :type Integer) (bFromSweep :type Boolean) (SweepResult :type "HitResult Structure (by ref)"))
  ;[1 1 1] 有BUG，得改
  (`self.掉落声音`))

(fn `UserConstructionScript`)