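; 门_BP is a door that swings open and closed when its 拾取物品 (pick up item) event fires.
; A FlipFlop alternates between playing and reversing a timeline, which lerps the yaw of the 拾取模型 mesh between closed and a quarter turn.
; A DoOnce on the timeline update plays a creak sound at the door's location, and resets when the timeline finishes.
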(event `/Game/BP/pickup.拾取物品`
  (`/Engine/EditorBlueprintResources/StandardMacros.FlipFlop`
    (:`A`
      (bind (_direction _alpha) (`Timeline|时间轴_0` :!label _label)
        (:`Update`
          (`SceneComponent.K2_SetRelativeRotation` (`self.拾取模型`) (`KismetMathLibrary.MakeRotator` 0.0 0.0 (`KismetMathLibrary.Lerp` 0.0 90.0 _alpha)) false false)
          (`/Engine/EditorBlueprintResources/StandardMacros.DoOnce` false :!label _label_2
            (:`Completed`
              (`GameplayStatics.PlaySoundAtLocation` "/Game/资产/音频/音效/橱柜吱吱_Cue.橱柜吱吱_Cue" (`self.K2_GetActorLocation`) (struct) 1.0 1.0 0.0 null null null))))
        (:`Finished`
          (goto _label_2 :!via `Reset`))))
    (:`B`
      (goto _label :!via `Reverse`))))

(fn `UserConstructionScript`
  (`parent.UserConstructionScript`))