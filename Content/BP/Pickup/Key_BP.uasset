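; Key_BP is a key item that the third-person player character can pick up.
; On BeginPlay it runs the parent logic, then caches the player pawn as a ThirdPersonCharacter.
; Its 拾取物品 (pick up item) event calls the character's 拾取物品到拾取位 to move it to the pickup slot, passing itself and item info named "Key".
; Overlap and Tick events are disabled stubs.
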(event `self.ReceiveBeginPlay`
  (`parent.ReceiveBeginPlay`)
  (bind _asthird_person_character (cast `/Game/BP/ThirdPersonBP/Blueprints/ThirdPersonCharacter` (`GameplayStatics.GetPlayerPawn` 0)))
  (set `self.Player` _asthird_person_character))

(event `/Game/BP/pickup.拾取物品`
  (`/Game/BP/ThirdPersonBP/Blueprints/ThirdPersonCharacter.拾取物品到拾取位` (`self.Player`) self "None" (make `/Game/BP/Pickup/物品信息` self "Key")))

(fn `UserConstructionScript`
  (`parent.UserConstructionScript`))