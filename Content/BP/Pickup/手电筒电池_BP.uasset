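; Flashlight battery pickup actor that adds one battery to the player's count when picked up.
; Its pickup event (拾取物品) casts the first player pawn to ThirdPersonCharacter, increments 手电筒电池数量 and destroys the actor.
; The construction script runs the parent's, then gives the pickup model a random world rotation, including roll, so placed batteries vary in orientation.
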(event `/Game/BP/pickup.拾取物品`
  (bind _asthird_person_character (cast `/Game/BP/ThirdPersonBP/Blueprints/ThirdPersonCharacter` (`GameplayStatics.GetPlayerPawn` 0)))
  (set `/Game/BP/ThirdPersonBP/Blueprints/ThirdPersonCharacter.手电筒电池数量` (+ (`/Game/BP/ThirdPersonBP/Blueprints/ThirdPersonCharacter.手电筒电池数量` _asthird_person_character) 1) _asthird_person_character)
  (`self.K2_DestroyActor`))

(fn `UserConstructionScript`
  (`parent.UserConstructionScript`)
  (`SceneComponent.K2_SetWorldRotation` (`self.拾取模型`) (`KismetMathLibrary.RandomRotator` true) false false))