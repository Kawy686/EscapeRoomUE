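; Bed Blueprint that the player character can get into and out of by switching possession.
; Box overlap enables interaction and opens a gate; leaving disables interaction and closes it.
; Each gated interact event plays force feedback and alternates via FlipFlop between possessing the bed and restoring the character at the Arrow transform.
; The character's tags are set to "Not" while the bed is possessed and "Player" on return.
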(event `/Game/BP/Player/Player_Intelface.交互`
  (bind _returnvalue (`GameplayStatics.GetPlayerController` 0))
  (bind (_returnvalue_location _returnvalue_rotation) (`KismetMathLibrary.BreakTransform` (`SceneComponent.K2_GetComponentToWorld` (`self.Arrow`))))
  (`PlayerController.K2_ClientPlayForceFeedback` (`GameplayStatics.GetPlayerController` 0) "/Game/手柄适配/FFE_2短.FFE_2短" "None" false false false)
  (`/Engine/EditorBlueprintResources/StandardMacros.Gate` true :!label _label
    (:`Exit`
      (`/Engine/EditorBlueprintResources/StandardMacros.FlipFlop`
        (:`A`
          (`Controller.Possess` _returnvalue self)
          (set `Actor.Tags` (`|MakeArray` "Not") (stale `self.Box.OnComponentBeginOverlap` _asthird_person_character)))
        (:`B`
          (`self.K2_SetActorLocationAndRotation` (stale `self.Box.OnComponentBeginOverlap` _asthird_person_character) _returnvalue_location _returnvalue_rotation false false)
          (`Controller.Possess` _returnvalue (stale `self.Box.OnComponentBeginOverlap` _asthird_person_character))
          (set `Actor.Tags` (`|MakeArray` "Player") (stale `self.Box.OnComponentBeginOverlap` _asthird_person_character)))))))

(event `self.Box.OnComponentBeginOverlap`
  (params (OverlappedComponent :type "PrimitiveComponent Object Reference") (OtherActor :type "Actor Object Reference") (OtherComp :type "PrimitiveComponent Object Reference") (OtherBodyIndex :type Integer) (bFromSweep :type Boolean) (SweepResult :type "HitResult Structure (by ref)"))
  (bind _asthird_person_character (`/Game/BP/PlayerFunctionLibrary.启用交互` self OtherActor))
  (goto _label :!via `Open`))

(event `self.Box.OnComponentEndOverlap`
  (params (OverlappedComponent :type "PrimitiveComponent Object Reference") (OtherActor :type "Actor Object Reference") (OtherComp :type "PrimitiveComponent Object Reference") (OtherBodyIndex :type Integer))
  (`/Game/BP/PlayerFunctionLibrary.禁用交互` OtherActor)
  (goto _label :!via `Close`))

(fn `UserConstructionScript`)